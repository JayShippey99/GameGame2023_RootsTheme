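; BP_Lumberjack is a flipbook-sprite enemy character that travels along the level's SplineBP path and destroys itself at the end.
; BeginPlay sets speed, tree damage and health by Type, then a timeline moves it along the spline, with Speed acting as travel duration.
; Tick picks a side or back flipbook from X velocity, flips control rotation and faces the GameInstance camera.
; Axis inputs also add movement; damage and health go unused here.
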(event Custom|Move%20Object
  ;[1 1 1] Enemy Moving along spline
  (Components|Timeline|SetPlayRate (Variables|Default|GetMoveThing) (/ 1.0 (Variables|Default|Getspeed)))
  (bind _newtrack_0 (Timeline|MoveThing Play)
    (:Update
      (Transformation|SetActorLocation (Spline|GetLocationatDistanceAlongSpline (Variables|/Game/Blueprints/EnemyStuff/SplineBP.SplineBP_C|GetSpline (Variables|Default|Getspline%20ref)) (Math|Float|Lerp 0.0 (Spline|GetSplineLength (Variables|/Game/Blueprints/EnemyStuff/SplineBP.SplineBP_C|GetSpline (Variables|Default|Getspline%20ref))) _newtrack_0) "World") false false))
    (:Finished
      (Development|PrintString "Deathhhhh")
      (Actor|DestroyActor)
      (Development|PrintString "dying"))))

(event Custom|updateControlRotation
  (Utilities|IsValid (Pawn|GetController)
    (:Is%20Valid
      (Math|Float|CompareFloat (.X (Math|Vector|BreakVector (Variables|/Script/Engine.MovementComponent|GetVelocity (Variables|Character|GetCharacterMovement)))) 0.0
        (:>
          (Pawn|SetControlRotation (Pawn|GetController) (Math|Rotator|MakeRotator 0.0 0.0 0.0)))
        (:<
          (Pawn|SetControlRotation (Pawn|GetController) (Math|Rotator|MakeRotator 0.0 0.0 1.8e+02)))))))

(event Custom|UpdateAnimation
  (Sprite|SetFlipbook (Variables|Default|GetSprite) (select (> (Math|Vector|VectorLength (Math|Vector|MakeVector (.x (Variables|/Script/Engine.MovementComponent|GetVelocity (Variables|Character|GetCharacterMovement))) 0.0 0.0)) 0.0) "/Game/SpriteAnimations/Sprites/Enemies/LumberJack/LumberSide/LumberSide.LumberSide" "/Game/SpriteAnimations/Sprites/Enemies/LumberJack/LumberBack/LumberBack.LumberBack")))

(event EventBeginPlay
  ;[1 1 1] Enemy types
  (Utilities|FlowControl|Delay 0.0)
  (Utilities|FlowControl|Sequence
    (:then_0
      (bind _returnvalue (Actor|GetActorOfClass "/Game/Blueprints/EnemyStuff/SplineBP.SplineBP_C"))
      (Variables|Default|Setspline%20ref _returnvalue)
      (switch int (Variables|Default|GetType)
        (:Default
          (Variables|Default|Setspeed 3e+01)
          (Variables|Default|SetDamageToTree 0)
          (Variables|Default|SetHealth 1.0))
        (:0
          (Variables|Default|Setspeed 5.0)
          (Variables|Default|SetDamageToTree 33)
          (Variables|Default|SetHealth 1.0))
        (:1
          (Variables|Default|Setspeed 3.0)
          (Variables|Default|SetDamageToTree 44)
          (Variables|Default|SetHealth 1.0))
        (:2
          (Variables|Default|Setspeed 1e+01)
          (Variables|Default|SetDamageToTree 55)
          (Variables|Default|SetHealth 1.0))
        (:3
          (Variables|Default|Setspeed 5.0)
          (Variables|Default|SetDamageToTree 69)
          (Variables|Default|SetHealth 1.0)))
      (CallFunction|MoveObject))
    (:then_1
      (bind _astdgame_instance (Utilities|Casting|CastToTDGameInstance (Game|GetGameInstance)))
      (Variables|Default|SetCameraRef (Variables|/Game/InstancesGameModesControllers/TDGameInstance.TDGameInstance_C|GetGameCamera _astdgame_instance)))))

(event EventTick
  (params (DeltaSeconds :type Float%20%28single-precision%29))
  (CallFunction|UpdateAnimation)
  (CallFunction|UpdateControlRotation)
  (CallFunction|FaceCamera (Variables|Default|GetCameraRef) self))

(event Input|AxisEvents|InputAxisx
  (params (AxisValue :type Float%20%28single-precision%29))
  (Pawn|Input|AddMovementInput "1.000000, 0, 0" AxisValue false))

(event Input|AxisEvents|InputAxisy
  (params (AxisValue :type Float%20%28single-precision%29))
  (Pawn|Input|AddMovementInput "0,1.000000, 0" AxisValue false))

(fn ConstructionScript)