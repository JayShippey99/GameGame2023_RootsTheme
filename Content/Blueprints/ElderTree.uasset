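; ElderTree is an actor with a health pool that enemy cubes damage on contact.
; When an EnemyCubeBP begins overlapping it, the tree subtracts that enemy's DamageToTree from TreeHealth.
; Tick polls TreeHealth every frame and destroys the actor once it reaches zero or below, with debug prints marking hits and death.
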(event EventTick
  (params (DeltaSeconds :type Float%20%28single-precision%29))
  (Development|PrintString (Utilities|String|ToString(Float) (Variables|Default|GetTreeHealth)) false false "(R=0.000000,G=0.660000,B=1.000000,A=1.000000)" 1e+01)
  (if (<= (Variables|Default|GetTreeHealth) 0.0)
    (Development|PrintString "treeDead")
    (Actor|DestroyActor)))

(event Collision|EventActorBeginOverlap
  (params (OtherActor :type Actor%20Object%20Reference))
  (bind _asenemy_cube_bp (Utilities|Casting|CastToEnemyCubeBP OtherActor))
  (Development|PrintString "TreeHit")
  (Variables|Default|SetTreeHealth (- (Variables|Default|GetTreeHealth) (Math|Conversions|ToFloat(Integer) (Variables|/Game/Blueprints/EnemyStuff/EnemyCubeBP.EnemyCubeBP_C|GetDamageToTree _asenemy_cube_bp)))))

(fn ConstructionScript)