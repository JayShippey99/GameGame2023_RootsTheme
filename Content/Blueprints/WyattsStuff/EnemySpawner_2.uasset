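; Enemy spawner actor that spawns a timed burst of AI enemies of the configured class at its own location.
; Tick watches the WillStart flag, calls SpawnEnemy when it is set, then clears it.
; SpawnEnemy re-calls itself after a short delay, incrementing CurrentAmount until it equals MaxAmount.
; The limit check follows each spawn, so one more enemy appears after the counter reaches the maximum.
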(event Custom|SpawnEnemy
  (AI|SpawnAIFromClass "/Game/Blueprints/WyattsStuff/Enemy.Enemy_C" 0 (Transformation|GetActorLocation) "0, 0, 0" false 0)
  (if (not (== (Variables|Default|GetCurrentAmount) (Variables|Default|GetMaxAmount)))
    (Variables|Default|SetCurrentAmount (+ (Variables|Default|GetCurrentAmount) 1))
    (Utilities|FlowControl|Delay 0.2)
    (CallFunction|SpawnEnemy)))

(event EventTick
  (params (DeltaSeconds :type Float%20%28single-precision%29))
  (if (Variables|Default|GetWillStart)
    (CallFunction|SpawnEnemy)
    (Variables|Default|SetWillStart false)))

(fn ConstructionScript)