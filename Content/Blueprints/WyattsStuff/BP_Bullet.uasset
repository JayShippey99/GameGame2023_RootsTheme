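; BP_Bullet is a projectile fired by tree towers at lumberjack enemies.
; Its construction script sets speed and picks the sprite from the AttackTreeData table, using Type as the row index.
; On overlap, type 3 (goo) calls ChangeSpeed on the lumberjack and persists, while other types apply damage and destroy the bullet.
; The bullet also destroys itself when it stops overlapping its parent tower, limiting its range.
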(event OnComponentBeginOverlap(Box)
  (params (OverlappedComponent :type Primitive%20Component%20Object%20Reference) (OtherActor :type Actor%20Object%20Reference) (OtherComp :type Primitive%20Component%20Object%20Reference) (OtherBodyIndex :type Integer) (bFromSweep :type Boolean) (SweepResult :type Hit%20Result%20Structure%20%28by%20ref%29))
  (bind _damage (Variables|Default|GetDamage))
  (bind _asbp_lumberjack (Utilities|Casting|CastToBP_Lumberjack OtherActor))
  (if (== (Variables|Default|GetType) 3)
    (Development|PrintString "Goo enemy!" false false)
    (Default|ChangeSpeed _asbp_lumberjack)
    (else
      (Development|PrintString (Utilities|String|ToString(Float) _damage))
      (Game|Damage|ApplyDamage _asbp_lumberjack _damage 0 0)
      (Actor|DestroyActor))))

(event Collision|EventActorEndOverlap
  (params (OtherActor :type Actor%20Object%20Reference))
  (bind _astree_tower (Utilities|Casting|CastToTreeTower OtherActor))
  (Development|PrintString (Utilities|String|Append (Utilities|String|ToString(Vector) (Variables|/Script/Engine.SceneComponent|GetRelativeScale3D (Variables|/Game/Blueprints/JaysStuff/TreeTower.TreeTower_C|GetDecal _astree_tower))) "   " (Utilities|String|ToString(Float) (Variables|/Game/Blueprints/JaysStuff/TreeTower.TreeTower_C|GetFireRadius _astree_tower))) false false)
  (if (== _astree_tower (Variables|Default|GetParentObj))
    (Development|PrintString "Killing bullet" false false)
    (Actor|DestroyActor)))

(fn ConstructionScript
  (bind _sprite (CallFunction|GetSprite (Variables|Default|GetType)))
  (Rendering|Components|Sprite|SetSprite (Variables|Default|GetPaperSprite) _sprite)
  (Variables|/Script/Engine.ProjectileMovementComponent|SetInitialSpeed (Variables|Default|GetProjectileMovement) (Variables|Default|GetSpeed)))

(fn GetSprite
  (params (Type :type Integer))
  (bind _outrownames (DataTable|GetDataTableRowNames "/Game/Utilities/AttackTreeData.AttackTreeData"))
  (bind _returnvalue (Utilities|GetDataTableRow "/Game/Utilities/AttackTreeData.AttackTreeData" (Utilities|Array|Get(acopy) _outrownames Type))
    (:then
      (return (.BulletSprite (Utilities|Struct|BreakAttackTreeUnitLevels _returnvalue))))))