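; Enemy spawner actor that releases a wave of AI enemies at its own location when play begins.
; SpawnEnemy calls itself on a short delay, incrementing a counter after each spawn until it reaches MaxAmount.
; After the last spawn it waits 30 seconds, then sets WillStart on the EnemySpawner_2 found in the level, handing off to that spawner.
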(event Custom|SpawnEnemy
  (AI|SpawnAIFromClass "/Game/Blueprints/WyattsStuff/Enemy.Enemy_C" 0 (Transformation|GetActorLocation) "0, 0, 0" false 0)
  (if (== (Variables|Default|GetCurrentAmount) (Variables|Default|GetMaxAmount))
    (Utilities|FlowControl|Delay 3e+01)
    (bind _returnvalue (Actor|GetActorOfClass "/Game/Blueprints/WyattsStuff/EnemySpawner_2.EnemySpawner_2_C"))
    (Variables|/Game/Blueprints/WyattsStuff/EnemySpawner_2.EnemySpawner_2_C|SetWillStart _returnvalue true)
    (else
      (Variables|Default|SetCurrentAmount (+ (Variables|Default|GetCurrentAmount) 1))
      (Utilities|FlowControl|Delay 0.2)
      (CallFunction|SpawnEnemy))))

(event EventBeginPlay
  (CallFunction|SpawnEnemy))

(fn ConstructionScript)