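; JayEnemy is an enemy that targets a Goal actor and damages the player's tower.
; Shortly after BeginPlay it sets its CharacterMovement walk speed to zero, then issues an AIMoveTo toward the first Goal found.
; Both move success and failure subtract a fixed amount from TowerHealth on the player's BP_TowerPawn, then destroy the enemy after a delay.
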(event EventBeginPlay
  (Utilities|FlowControl|Delay 0.2)
  (Variables|/Script/Engine.CharacterMovementComponent|SetMaxWalkSpeed (Variables|Character|GetCharacterMovement) 0.0)
  (bind _outactors (Actor|GetAllActorsOfClass "/Game/Blueprints/WyattsStuff/Goal.Goal_C"))
  (AI|AIMoveTo self "0, 0, 0" (Utilities|Array|Get(acopy) _outactors) 5.0 false
    (:OnSuccess
      _)
    (:OnFail
      _))
  (bind _asbp_tower_pawn_c (Utilities|Casting|CastToBP_TowerPawnC (Game|Player|GetPlayerPawn 0)))
  (Variables|/Game/Blueprints/WyattsStuff/BP_TowerPawnC.BP_TowerPawnC_C|SetTowerHealth _asbp_tower_pawn_c (- (Variables|/Game/Blueprints/WyattsStuff/BP_TowerPawnC.BP_TowerPawnC_C|GetTowerHealth _asbp_tower_pawn_c) 1e+01))
  (Utilities|FlowControl|Delay 3.0)
  (Actor|DestroyActor))

(fn ConstructionScript
  (|CallParentFunction))