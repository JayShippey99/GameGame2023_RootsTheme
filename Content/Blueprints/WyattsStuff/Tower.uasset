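; Tower defense turret that turns toward the nearest EnemyBase actor and fires at enemies within 500 units.
; A self-repeating 0.2-second loop finds the closest enemy, then checks range against it but validity and death against the first enemy found.
; Shoot spawns a BP_Bullet at the tower and returns the first bullet found, which is destroyed immediately.
; Damage's health reduction is disconnected, so it deals none.
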(event Custom|GetClosesetEnemy
  (CallFunction|ClosestCharacter)
  (bind _outactors (Actor|GetAllActorsOfClass "/Game/Blueprints/WyattsStuff/EnemyBase.EnemyBase_C"))
  (Utilities|IsValid (Utilities|Array|Get(acopy) _outactors)
    (:Is%20Valid
      (if (<= (Transformation|GetDistanceTo (Variables|Default|GetClosestEnemy)) 5e+02)
        (if (Variables|/Game/Blueprints/WyattsStuff/EnemyBase.EnemyBase_C|GetisDead (Utilities|Array|Get(acopy) _outactors))
          _
          (else
            (bind _returnvalue (CallFunction|Shoot))
            (CallFunction|Damage)
            (Actor|DestroyActor _returnvalue)))))
    (:Is%20Not%20Valid
      _))
  (Utilities|FlowControl|Delay 0.2)
  (CallFunction|GetClosesetEnemy))

(event EventBeginPlay
  (Utilities|FlowControl|Sequence
    (:then_0
      (bind _outactors (Actor|GetAllActorsOfClass "/Game/Blueprints/WyattsStuff/EnemyBase.EnemyBase_C"))
      (for _array_element _outactors
        (Utilities|Array|Add (Variables|Default|GetEnemy) _array_element)))
    (:then_1
      (Utilities|FlowControl|Delay 0.2)
      (CallFunction|GetClosesetEnemy))))

(fn ConstructionScript
  (|CallParentFunction))

(fn Shoot
  (bind _outactors (Actor|GetAllActorsOfClass "/Game/Blueprints/WyattsStuff/EnemyBase.EnemyBase_C"))
  (Utilities|IsValid (Utilities|Array|Get(acopy) _outactors)
    (:Is%20Valid
      (Game|SpawnActorfromClass "/Game/Blueprints/WyattsStuff/BP_Bullet.BP_Bullet_C" (Math|Transform|MakeTransform (Transformation|GetActorLocation) "0, 0, 0" "1,1,1") "Undefined" 0 0 0.0 0)
      (bind _returnvalue (Actor|GetActorOfClass "/Game/Blueprints/WyattsStuff/BP_Bullet.BP_Bullet_C"))
      (return _returnvalue))))

(fn Damage
  (bind _outactors (Actor|GetAllActorsOfClass "/Game/Blueprints/WyattsStuff/EnemyBase.EnemyBase_C")))

(fn ClosestCharacter
  (bind _outactors (Actor|GetAllActorsOfClass "/Game/Blueprints/WyattsStuff/EnemyBase.EnemyBase_C"))
  (for _array_element _outactors
    (Utilities|Array|AppendArray (Variables|Default|GetEnemyDistance) (Utilities|Array|MakeArray (Transformation|GetDistanceTo _array_element))))
  (Variables|Default|SetClosestEnemy (Utilities|Array|Get(acopy) _outactors (.IndexOfMinValue (Math|Float|MinOfFloatArray (Variables|Default|GetEnemyDistance)))))
  (Transformation|SetActorRotation (Math|Rotator|MakeRotator 0.0 0.0 (.yaw (Class|KismetMathLibrary|RInterptoConstant (Transformation|GetActorRotation) (Math|Rotator|FindLookatRotation (Transformation|GetActorLocation) (Transformation|GetActorLocation (Utilities|Array|Get(acopy) _outactors (.IndexOfMinValue (Math|Float|MinOfFloatArray (Variables|Default|GetEnemyDistance)))))) (Utilities|Time|GetWorldDeltaSeconds) 0.0))))
  (Utilities|Array|Clear (Variables|Default|GetEnemyDistance)))