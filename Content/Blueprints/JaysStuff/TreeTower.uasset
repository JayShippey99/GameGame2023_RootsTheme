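; Paper2D tree tower for a tower defense game that auto-fires at spline enemies.
; While dragged it follows a mouse trace, wiggles toward the camera and tints over TreeDenierZones, where dropping destroys it.
; Once placed, a FireRate loop shoots the closest enemy in range using Type-specific bullet patterns.
; AttackTreeData supplies stats and sprites per Age, which advances at round end; type 4 gains damage from nearby towers at round start.
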(event Custom|GetClosesetEnemy
  (CallFunction|FindClosestCharacter)
  (bind _outactors (Actor|GetAllActorsOfClass "/Game/Blueprints/EnemyStuff/JaySplineEnemy.JaySplineEnemy_C"))
  (Utilities|IsValid (Utilities|Array|Get(acopy) _outactors)
    (:Is%20Valid
      (if (<= (Transformation|GetDistanceTo (Variables|Default|GetClosestEnemy)) (* 100 (Variables|Default|GetFireRadius)))
        (CallFunction|Shoot)
        (Development|PrintString "SHOOT")))
    (:Is%20Not%20Valid
      _))
  (Utilities|FlowControl|Delay (Variables|Default|GetFireRate))
  (CallFunction|GetClosesetEnemy))

(event EventBeginPlay
  (Utilities|FlowControl|Delay 0.0)
  (bind _astdgame_instance (Utilities|Casting|CastToTDGameInstance (Game|GetGameInstance)))
  (Variables|Default|SetCameraRef (Variables|/Game/InstancesGameModesControllers/TDGameInstance.TDGameInstance_C|GetGameCamera _astdgame_instance))
  (CallFunction|GetOlder))

(event Collision|EventActorBeginOverlap
  (params (OtherActor :type Actor%20Object%20Reference))
  (bind _asjay_spline_enemy (Utilities|Casting|CastToJaySplineEnemy OtherActor))
  (Variables|Default|SetClosestEnemy _asjay_spline_enemy))

(event EventTick
  (params (DeltaSeconds :type Float%20%28single-precision%29))
  (bind _returnvalue (Transformation|GetActorLocation))
  (bind _cameraref (Variables|Default|GetCameraRef))
  (bind _returnvalue_2 (Transformation|GetActorLocation _cameraref))
  (bind _returnvalue_3 (Math|Rotator|FindLookatRotation _returnvalue_2 _returnvalue))
  (if (Variables|Default|GetDragging)
    (bind _wiggle (Timeline|Wiggle Play)
      (:Update
        (Transformation|SetActorRotation (Math|Rotator|MakeRotator (+ (* 2 _wiggle) (.roll _returnvalue_3)) (+ (.pitch _returnvalue_3) 15.0) 0.0))
        (CallFunction|Draggin)))
    (else
      (Utilities|FlowControl|DoOnce false
        (:Completed
          (CallFunction|GetClosesetEnemy)
          (Timeline|Wiggle Stop))))))

(fn ConstructionScript
  (bind _newparam (CallFunction|GetAgeStats))
  (Variables|Default|SetFireRadius (.Range (Utilities|Struct|BreakAttackTreeUnitStruct _newparam)))
  (Variables|Default|SetFireRate (.Attackrate (Utilities|Struct|BreakAttackTreeUnitStruct _newparam)))
  (CallFunction|SetVisibleRadius)
  (Rendering|Components|Sprite|SetSprite (Variables|Default|GetPaperSprite) (.Sprite (Utilities|Struct|BreakAttackTreeUnitStruct _newparam))))

(fn Place
  (if (Variables|Default|GetCannotPlace)
    (Actor|DestroyActor)
    (else
      (Variables|Default|SetDragging false)
      (CallFunction|MatchCameraAngle))))

(fn Draggin
  (bind _returnvalue (Game|GetPlayerController 0))
  (bind _papersprite (Variables|Default|GetPaperSprite))
  (bind (_worldlocation _worlddirection) (Game|Player|ConvertMouseLocationToWorldSpace _returnvalue))
  (bind _outhit (Collision|LineTraceByChannel (Transformation|GetActorLocation (Variables|Default|GetCameraRef)) (+ _worldlocation (* _worlddirection 1e+04)) "TraceTypeQuery1" false 0 "None" false))
  (Transformation|SetActorLocation (.Location (Collision|BreakHitResult _outhit)) false false)
  (Utilities|Casting|CastToTreeDenierZone (.HitActor (Collision|BreakHitResult _outhit))
    (:then
      (Sprite|SetSpriteColor _papersprite (Variables|Default|GetCannotPlaceColor))
      (Variables|Default|SetCannotPlace true))
    (:CastFailed
      (Sprite|SetSpriteColor _papersprite (Variables|Default|GetCanPlaceColor))
      (Variables|Default|SetCannotPlace false))))

(fn MatchCameraAngle
  (Transformation|SetActorRotation (Math|Rotator|MakeRotator 0.0 (+ (.pitch (Math|Rotator|FindLookatRotation (Transformation|GetActorLocation (Variables|Default|GetCameraRef)) (Transformation|GetActorLocation))) 15.0) 0.0)))

(fn Shoot
  (bind _returnvalue (Transformation|GetActorLocation))
  (bind _closestenemy (Variables|Default|GetClosestEnemy))
  (bind _returnvalue_2 (Transformation|GetActorLocation _closestenemy))
  (bind _returnvalue_3 (Math|Rotator|FindLookatRotation _returnvalue _returnvalue_2))
  (if (> (Variables|Default|GetAge) 0)
    (Utilities|IsValid _closestenemy
      (:Is%20Valid
        (switch int (Variables|Default|GetType)
          (:0
            (CallFunction|ShootLikePine _returnvalue_3))
          (:1
            (CallFunction|ShootLikeWalnut _returnvalue_3))
          (:2
            (CallFunction|ShootLikePalm _returnvalue_3))
          (:3
            (CallFunction|ShootLikeMaple _returnvalue_3)))))))

(fn DoDamage)

(fn FindClosestCharacter
  (bind _outactors (Actor|GetAllActorsOfClass "/Game/Blueprints/EnemyStuff/JaySplineEnemy.JaySplineEnemy_C"))
  (for _array_element _outactors
    (Utilities|Array|AppendArray (Variables|Default|GetEnemyDistance) (Utilities|Array|MakeArray (Transformation|GetDistanceTo _array_element))))
  (Variables|Default|SetClosestEnemy (Utilities|Array|Get(acopy) _outactors (.IndexOfMinValue (Math|Float|MinOfFloatArray (Variables|Default|GetEnemyDistance)))))
  ;[1 1 1] After each frame clear the distances, cause they change
  (Utilities|Array|Clear (Variables|Default|GetEnemyDistance)))

(fn SetVisibleRadius
  (bind _fireradius (Variables|Default|GetFireRadius))
  (Transformation|SetRelativeScale3D (Variables|Default|GetDecal) (Math|Conversions|ToVector(Float) _fireradius))
  (Transformation|SetRelativeScale3D (Variables|Default|GetShootRadius) (Math|Conversions|ToVector(Float) _fireradius)))

(fn GetOlder
  (Math|Integer|IncrementInt (Variables|Default|GetAge)
    (:%20%20
      (bind _outrownames (DataTable|GetDataTableRowNames "/Game/Utilities/AttackTreeData.AttackTreeData"))
      (bind _returnvalue (Utilities|GetDataTableRow "/Game/Utilities/AttackTreeData.AttackTreeData" (Utilities|Array|Get(acopy) _outrownames (Variables|Default|GetType)))
        (:then
          (switch int (Variables|Default|GetAge)
            (:0
              (LocalVariables|SetnewStats (.Level1 (Utilities|Struct|BreakAttackTreeUnitLevels _returnvalue))))
            (:1
              (LocalVariables|SetnewStats (.Level2 (Utilities|Struct|BreakAttackTreeUnitLevels _returnvalue))))
            (:2
              (LocalVariables|SetnewStats (.Level3 (Utilities|Struct|BreakAttackTreeUnitLevels _returnvalue)))
              (Transformation|SetActorScale3D (* (Transformation|GetActorScale3D) 1.5))))
          (Rendering|Components|Sprite|SetSprite (Variables|Default|GetPaperSprite) (.Sprite (Utilities|Struct|BreakAttackTreeUnitStruct (LocalVariables|GetnewStats))))
          (Variables|Default|SetDamage (.Damage (Utilities|Struct|BreakAttackTreeUnitStruct (LocalVariables|GetnewStats))))
          (Variables|Default|SetFireRadius (.Range (Utilities|Struct|BreakAttackTreeUnitStruct (LocalVariables|GetnewStats))))
          (Variables|Default|SetFireRate (.Attackrate (Utilities|Struct|BreakAttackTreeUnitStruct (LocalVariables|GetnewStats)))))))))

(fn RedWoodBuff
  (bind _newparam (CallFunction|GetAgeStats (Variables|Default|GetAge)))
  (Variables|Default|SetDamage (.Damage (Utilities|Struct|BreakAttackTreeUnitStruct _newparam)))
  (bind _outactors (Actor|GetAllActorsOfClass "TreeTower_C"))
  (for _array_element _outactors
    (if (and (== (Variables|Default|GetType) 4) (< (Math|Vector|Distance(Vector) (Transformation|GetActorLocation) (Transformation|GetActorLocation _array_element)) (* 100 (Variables|Default|GetFireRadius))))
      (Variables|Default|SetDamage (+ (Variables|Default|GetDamageBonus) (Variables|Default|GetDamage))))))

(fn GetAgeStats
  (params (Age :type Integer))
  (bind _outrownames (DataTable|GetDataTableRowNames "/Game/Utilities/AttackTreeData.AttackTreeData"))
  (bind _returnvalue (Utilities|GetDataTableRow "/Game/Utilities/AttackTreeData.AttackTreeData" (Utilities|Array|Get(acopy) _outrownames (Variables|Default|GetType)))
    (:then
      (switch int Age
        (:0
          (return (.Level1 (Utilities|Struct|BreakAttackTreeUnitLevels _returnvalue))))
        (:1
          (return (.Level2 (Utilities|Struct|BreakAttackTreeUnitLevels _returnvalue))))
        (:2
          (return (.Level3 (Utilities|Struct|BreakAttackTreeUnitLevels _returnvalue))))))))

(fn EndOfRoundFunctions
  (CallFunction|GetOlder))

(fn BeginningOfRoundFunctions
  (CallFunction|RedWoodBuff))

(fn ShootLikePine
  (params (Angle :type Rotator))
  (Game|SpawnActorfromClass "/Game/Blueprints/WyattsStuff/BP_Bullet.BP_Bullet_C" (Math|Transform|MakeTransform (+ (Transformation|GetWorldLocation (Variables|Default|GetShootLocation)) "0, 0, 0") Angle "1,1,1") "Undefined" 0 (Variables|Default|GetCameraRef) 5e+03 (Variables|Default|GetType) self 0.0 0))

(fn ShootLikeWalnut
  (params (Angle :type Rotator))
  (bind (_roll _pitch _yaw) (Math|Rotator|BreakRotator Angle))
  (bind (_roll_2 _pitch_2 _yaw_2) (Math|Rotator|BreakRotator Angle))
  (Game|SpawnActorfromClass "/Game/Blueprints/WyattsStuff/BP_Bullet.BP_Bullet_C" (Math|Transform|MakeTransform (+ (Transformation|GetWorldLocation (Variables|Default|GetShootLocation)) "0, 0, 0") Angle "0.500000,0.500000,0.500000") "Undefined" 0 (Variables|Default|GetCameraRef) 4e+03 (Variables|Default|GetType) self 0.0 0)
  (Game|SpawnActorfromClass "/Game/Blueprints/WyattsStuff/BP_Bullet.BP_Bullet_C" (Math|Transform|MakeTransform (+ (Transformation|GetWorldLocation (Variables|Default|GetShootLocation)) "0, 0, 0") (Math|Rotator|MakeRotator _roll_2 _pitch_2 (+ _yaw_2 45.0)) "0.500000,0.500000,0.500000") "Undefined" 0 (Variables|Default|GetCameraRef) 4e+03 (Variables|Default|GetType) self 0.0 0)
  (Game|SpawnActorfromClass "/Game/Blueprints/WyattsStuff/BP_Bullet.BP_Bullet_C" (Math|Transform|MakeTransform (+ (Transformation|GetWorldLocation (Variables|Default|GetShootLocation)) "0, 0, 0") (Math|Rotator|MakeRotator _roll _pitch (- _yaw 45.0)) "0.500000,0.500000,0.500000") "Undefined" 0 (Variables|Default|GetCameraRef) 4e+03 (Variables|Default|GetType) self 0.0 0))

(fn ShootLikePalm
  (params (Angle :type Rotator))
  (Game|SpawnActorfromClass "/Game/Blueprints/WyattsStuff/BP_Bullet.BP_Bullet_C" (Math|Transform|MakeTransform (+ (Transformation|GetWorldLocation (Variables|Default|GetShootLocation)) "0, 0, 0") Angle "1,1,1") "Undefined" 0 (Variables|Default|GetCameraRef) 2e+03 (Variables|Default|GetType) self 0.0 0))

(fn ShootLikeMaple
  (params (Angle :type Rotator))
  (Game|SpawnActorfromClass "/Game/Blueprints/WyattsStuff/BP_Bullet.BP_Bullet_C" (Math|Transform|MakeTransform (+ (Transformation|GetWorldLocation (Variables|Default|GetShootLocation)) "0, 0, 0") Angle "0.700000,0.700000,0.700000") "Undefined" 0 (Variables|Default|GetCameraRef) 5e+03 (Variables|Default|GetType) self 0.0 0))