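; Spline-following enemy for what appears to be a tower defense game, with per-type speed, health and tree damage set at BeginPlay.
; A timeline lerps it along the first SplineBP found, with play rate 1/Speed, so higher Speed values move slower.
; Each tick it faces the game instance's camera and destroys itself at zero health.
; Reaching the spline's end also destroys it, without applying DamageToTree here.
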(event Custom|Move%20Object
  ;[1 1 1] Enemy Moving along spline
  (Components|Timeline|SetPlayRate (Variables|Default|GetmoveObject%20T) (/ 1.0 (Variables|Default|Getspeed)))
  (bind _move_track (Timeline|moveObject%20T Play)
    (:Update
      (Transformation|SetActorLocation (Spline|GetLocationatDistanceAlongSpline (Variables|/Game/Blueprints/EnemyStuff/SplineBP.SplineBP_C|GetSpline (Variables|Default|Getspline%20ref)) (Math|Float|Lerp 0.0 (Spline|GetSplineLength (Variables|/Game/Blueprints/EnemyStuff/SplineBP.SplineBP_C|GetSpline (Variables|Default|Getspline%20ref))) _move_track) "World") false false))
    (:Finished
      (Development|PrintString "Deathhhhh")
      (Actor|DestroyActor)
      (Development|PrintString "dying"))))

(event EventBeginPlay
  ;[1 1 1] Enemy types
  (Utilities|FlowControl|Delay 0.0)
  (Utilities|FlowControl|Sequence
    (:then_0
      (Input|EnableInput (Game|GetPlayerController 0))
      (bind _returnvalue (Actor|GetActorOfClass "/Game/Blueprints/EnemyStuff/SplineBP.SplineBP_C"))
      (Variables|Default|Setspline%20ref _returnvalue)
      (switch int (Variables|Default|Gettype)
        (:Default
          (Variables|Default|Setspeed 1e+02)
          (Variables|Default|SetDamageToTree 0)
          (Variables|Default|SetHealth 1.0))
        (:0
          (Variables|Default|Setspeed 5.0)
          (Variables|Default|SetDamageToTree 33)
          (Variables|Default|SetHealth 1.0))
        (:1
          (Variables|Default|Setspeed 3.0)
          (Variables|Default|SetDamageToTree 44)
          (Variables|Default|SetHealth 1.0))
        (:2
          (Variables|Default|Setspeed 1e+01)
          (Variables|Default|SetDamageToTree 55)
          (Variables|Default|SetHealth 1.0))
        (:3
          (Variables|Default|Setspeed 5.0)
          (Variables|Default|SetDamageToTree 69)
          (Variables|Default|SetHealth 1.0)))
      (CallFunction|MoveObject))
    (:then_1
      (bind _astdgame_instance (Utilities|Casting|CastToTDGameInstance (Game|GetGameInstance)))
      (Variables|Default|SetCameraRef (Variables|/Game/InstancesGameModesControllers/TDGameInstance.TDGameInstance_C|GetGameCamera _astdgame_instance)))))

(event EventTick
  (params (DeltaSeconds :type Float%20%28single-precision%29))
  (CallFunction|FaceCamera (Variables|Default|GetCameraRef) self)
  (CallFunction|CheckifDead))

(fn ConstructionScript)

(fn CheckifDead
  (if (<= (Variables|Default|GetHealth) 0.0)
    (Development|PrintString "I DIED")
    (Actor|DestroyActor)))