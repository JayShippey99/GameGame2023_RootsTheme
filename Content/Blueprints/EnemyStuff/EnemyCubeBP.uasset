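; Enemy cube actor that travels along the level's SplineBP path, with a Type that sets its speed, tree damage and health at BeginPlay.
; A timeline scaled by Speed lerps distance along the spline to set location and rotation, and destroys the cube when it finishes.
; Tick also destroys it when Health runs out, but the health decrement and ApplyDamage nodes are disconnected and never run.
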(event Custom|Move%20Object
  (bind _spline_ref (Variables|Default|Getspline%20ref))
  (bind _spline (Variables|/Game/Blueprints/EnemyStuff/SplineBP.SplineBP_C|GetSpline _spline_ref))
  ;[1 1 1] Enemy Moving along spline
  (Components|Timeline|SetPlayRate (Variables|Default|GetmoveObject%20T) (/ 1.0 (Variables|Default|Getspeed)))
  (bind _move_track (Timeline|moveObject%20T Play)
    (:Update
      (Transformation|SetActorTransform (Math|Transform|MakeTransform (Spline|GetLocationatDistanceAlongSpline _spline (Math|Float|Lerp 0.0 (Spline|GetSplineLength (Variables|/Game/Blueprints/EnemyStuff/SplineBP.SplineBP_C|GetSpline (Variables|Default|Getspline%20ref))) _move_track) "World") (Spline|GetRotationatDistanceAlongSpline _spline (Math|Float|Lerp 0.0 (Spline|GetSplineLength (Variables|/Game/Blueprints/EnemyStuff/SplineBP.SplineBP_C|GetSpline (Variables|Default|Getspline%20ref))) _move_track) "Local") "1,1,1")))
    (:Finished
      (Development|PrintString "Deathhhhh")
      (Actor|DestroyActor))))

(event EventBeginPlay
  ;[1 1 1] Enemy types
  (bind _returnvalue (Actor|GetActorOfClass "/Game/Blueprints/EnemyStuff/SplineBP.SplineBP_C"))
  (Variables|Default|Setspline%20ref _returnvalue)
  (switch int (Variables|Default|Gettype)
    (:0
      (Variables|Default|Setspeed 5.0)
      (Variables|Default|SetDamageToTree 33)
      (Variables|Default|SetHealth 1.0))
    (:1
      (Variables|Default|Setspeed 5.0)
      (Variables|Default|SetDamageToTree 44)
      (Variables|Default|SetHealth 1.0))
    (:2
      (Variables|Default|Setspeed 5.0)
      (Variables|Default|SetDamageToTree 55)
      (Variables|Default|SetHealth 1.0))
    (:3
      (Variables|Default|Setspeed 5.0)
      (Variables|Default|SetDamageToTree 69)
      (Variables|Default|SetHealth 1.0)))
  (CallFunction|MoveObject))

(event EventTick
  (params (DeltaSeconds :type Float%20%28single-precision%29))
  ;[1 1 1] health stuff
  (if (<= (Variables|Default|GetHealth) 0.0)
    (Actor|DestroyActor)
    (Development|PrintString "noHealth")))

(fn ConstructionScript)