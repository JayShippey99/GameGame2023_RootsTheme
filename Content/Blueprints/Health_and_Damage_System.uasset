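; Actor Blueprint that prototypes a simple health and death system, with damage triggered by a key press.
; It prints Health on screen at BeginPlay, and each press of R decrements Health and prints the new value.
; Tick polls Health every frame and destroys the actor once it reaches zero or below.
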(event EventBeginPlay
  (Development|PrintString (Utilities|String|ToString(Float) (Variables|Default|GetHealth)) true true "(R=0.000000,G=0.660000,B=1.000000,A=1.000000)" 1e+01))

(event Collision|EventActorBeginOverlap
  (params (OtherActor :type Actor%20Object%20Reference)))

(event EventTick
  (params (DeltaSeconds :type Float%20%28single-precision%29))
  (if (<= (Variables|Default|GetHealth) 0.0)
    (Actor|DestroyActor)))

(event Input|KeyboardEvents|R
  (params (Key :type Key%20Structure :default "None"))
  (:Pressed
    (Math|Float|DecrementFloat (Variables|Default|GetHealth)
      (:%20%20
        (Development|PrintString (Utilities|String|ToString(Float) (Variables|Default|GetHealth)) true true "(R=0.000000,G=0.660000,B=1.000000,A=1.000000)" 1e+01)))))

(fn ConstructionScript)